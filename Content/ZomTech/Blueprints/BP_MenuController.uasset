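; BP_MenuController is the player controller for the menu, setting up the UI and cinematic backdrop on BeginPlay.
; For the local controller only, it adds the WB_Menu widget to the viewport, shows the mouse cursor and loops LS_MenuSequence endlessly.
; It then polls at short intervals until a CineCameraActor exists and sets it as the view target.
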(event EventBeginPlay
  ;[0 0 0] Begin Play - Create HUD
  (if (Pawn|IsLocalPlayerController)
    (bind _returnvalue (UserInterface|CreateWidget "/Game/ZomTech/Blueprints/Widgets/WB_Menu.WB_Menu_C"))
    (UserInterface|Viewport|AddtoViewport _returnvalue 0)
    (Variables|Default|SetbShowMouseCursor true)
    (bind _returnvalue_2 (Sequencer|Player|CreateLevelSequencePlayer "/Game/ZomTech/Sequence/LS_MenuSequence.LS_MenuSequence" (Utilities|Struct|MakeMovieSceneSequencePlaybackSettings true (Utilities|Struct|MakeMovieSceneSequenceLoopCount 0) 1.0 0.0 false false false false false false false false)))
    (Class|MovieSceneSequencePlayer|PlayLooping _returnvalue_2 -1)
    (bind _returnvalue_3 (Actor|GetActorOfClass "/Script/CinematicCamera.CineCameraActor" :!label _label))
    (Utilities|IsValid _returnvalue_3
      (:Is%20Valid
        (Game|Player|SetViewTargetwithBlend self _returnvalue_3 0.0 "VTBlend_Linear" 0.0 false))
      (:Is%20Not%20Valid
        (Utilities|FlowControl|Delay 0.1)
        (goto _label)))))

(fn ConstructionScript)