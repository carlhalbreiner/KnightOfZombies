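; Zombie AI Blueprint that passes incoming damage to its BPZombieAIComponent and plays physics-based hit reactions.
; Multicast hit events simulate bodies from spine_01 down the bone chain and apply an impulse at the hit bone, retrying until it simulates.
; Two chained timelines ease the physics blend weight up and back down, then disable simulation if still alive.
; When dead, hits stop both timelines before applying the impulse.
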(event Custom|Hit%20Reaction%20-%20Multicast
  (params (Hit%20Location :type Vector) (Hit%20Impulse :type Vector) (Bone :type Name))
  ;[0 0 0] Hit Reaction
  (if (or (!= Bone "root") (!= Bone "pelvis"))
    (Class|SkeletalMeshComponent|SetAllBodiesBelowSimulatePhysics (Variables|Character|GetMesh) (Utilities|Name|MakeLiteralName "spine_01") true true)
    (Class|SkeletalMeshComponent|SetPhysicsBlendWeight (Variables|Character|GetMesh) 0.0)
    (Utilities|FlowControl|DelayUntilNextTick)
    (Utilities|FlowControl|Sequence
      (:then_0
        (Utilities|FlowControl|Sequence
          (:then_0
            (bind _newtrack_0 (Timeline|Timeline_0 PlayFromStart)
              (:Update
                (if (> _newtrack_0 0.0)
                  (bind _output_get (Variables|Don'tEdit|SetPhysics (Math|Interpolation|FInterpTo (Variables|Don'tEdit|GetPhysics) 1.0 _newtrack_0 0.2)))
                  (Class|SkeletalMeshComponent|SetAllBodiesBelowPhysicsBlendWeight (Variables|Character|GetMesh) (Utilities|Name|MakeLiteralName "spine_01") _output_get false true)))
              (:Finished
                (bind _newtrack_0_2 (Timeline|Timeline_1 PlayFromStart)
                  (:Update
                    (bind _output_get_2 (Variables|Don'tEdit|SetPhysics (Math|Interpolation|FInterpTo (Variables|Don'tEdit|GetPhysics) 0.0 _newtrack_0_2 0.1)))
                    (Class|SkeletalMeshComponent|SetAllBodiesBelowPhysicsBlendWeight (Variables|Character|GetMesh) (Utilities|Name|MakeLiteralName "spine_01") _output_get_2 false true))
                  (:Finished
                    (if (not (Variables|/Game/ZomTech/Blueprints/Components/BP_Zombie_AI_Component.BP_Zombie_AI_Component_C|GetDead (Variables|Default|GetBP_Zombie_AI_Component)))
                      (Class|SkeletalMeshComponent|SetAllBodiesSimulatePhysics (Variables|Character|GetMesh) false)))))))
          (:then_1
            (Timeline|Timeline_1 Stop))))
      (:then_1
        (if (Physics|IsSimulatingPhysics (Variables|Character|GetMesh) Bone) :!label _label
          (Physics|AddImpulseatLocation (Variables|Character|GetMesh) Hit%20Impulse Hit%20Location Bone)
          (else
            (Utilities|FlowControl|RetriggerableDelay 0.1)
            (goto _label)))))))

(event Custom|HitReaction%20Dead%20-%20Multicast
  ;[0 0 0] Hit Reaction
  (Utilities|FlowControl|Sequence
    (:then_0
      (bind _newtrack_0 (Timeline|Timeline_0 Stop)
        (:Update
          (if (> _newtrack_0 0.0)
            (bind _output_get (Variables|Don'tEdit|SetPhysics (Math|Interpolation|FInterpTo (Variables|Don'tEdit|GetPhysics) 1.0 _newtrack_0 0.2)))
            (Class|SkeletalMeshComponent|SetAllBodiesBelowPhysicsBlendWeight (Variables|Character|GetMesh) (Utilities|Name|MakeLiteralName "spine_01") _output_get false true)))
        (:Finished
          (bind _newtrack_0_2 (Timeline|Timeline_1 PlayFromStart)
            (:Update
              (bind _output_get_2 (Variables|Don'tEdit|SetPhysics (Math|Interpolation|FInterpTo (Variables|Don'tEdit|GetPhysics) 0.0 _newtrack_0_2 0.1)))
              (Class|SkeletalMeshComponent|SetAllBodiesBelowPhysicsBlendWeight (Variables|Character|GetMesh) (Utilities|Name|MakeLiteralName "spine_01") _output_get_2 false true))
            (:Finished
              (if (not (Variables|/Game/ZomTech/Blueprints/Components/BP_Zombie_AI_Component.BP_Zombie_AI_Component_C|GetDead (Variables|Default|GetBP_Zombie_AI_Component)))
                (Class|SkeletalMeshComponent|SetAllBodiesSimulatePhysics (Variables|Character|GetMesh) false)))))))
    (:then_1
      (Timeline|Timeline_1 Stop))
    (:then_2
      (if (Physics|IsSimulatingPhysics (Variables|Character|GetMesh) (stale Custom|Hit%20Reaction%20-%20Multicast Bone)) :!label _label
        (Physics|AddImpulseatLocation (Variables|Character|GetMesh) (stale Custom|Hit%20Reaction%20-%20Multicast Hit%20Impulse) (stale Custom|Hit%20Reaction%20-%20Multicast Hit%20Location) (stale Custom|Hit%20Reaction%20-%20Multicast Bone))
        (else
          (Utilities|FlowControl|RetriggerableDelay 0.1)
          (goto _label))))))

(event Game|Damage|EventAnyDamage
  (params (Damage :type Float%20%28single-precision%29) (DamageType :type Damage%20Type%20Object%20Reference) (InstigatedBy :type Controller%20Object%20Reference) (DamageCauser :type Actor%20Object%20Reference))
  ;[0 0 0] Damage
  (if (not (Variables|/Game/ZomTech/Blueprints/Components/BP_Zombie_AI_Component.BP_Zombie_AI_Component_C|GetDead (Variables|Default|GetBP_Zombie_AI_Component)))
    (Default|DecreaseHealth (Variables|Default|GetBP_Zombie_AI_Component) Damage)))

(event EventHitReaction
  (params (Hit%20Location :type Vector :default "0, 0, 0") (Hit%20Impulse :type Vector :default "0, 0, 0") (Bone :type Name :default "None"))
  ;[0 0 0] Hit Reaction
  (if (Variables|/Game/ZomTech/Blueprints/Components/BP_Zombie_AI_Component.BP_Zombie_AI_Component_C|GetDead (Variables|Default|GetBP_Zombie_AI_Component))
    (CallFunction|HitReactionDead-Multicast)
    (else
      (CallFunction|HitReaction-Multicast Hit%20Location Hit%20Impulse Bone))))

(fn ConstructionScript
  (Class|PhysicalAnimationComponent|SetSkeletalMeshComponent (Variables|Default|GetPhysicalAnimation) (Variables|Character|GetMesh)))