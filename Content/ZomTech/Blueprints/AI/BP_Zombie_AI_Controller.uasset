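; AI controller for zombies that runs BT_Zombie_AI and turns sight and hearing perception into blackboard targets and AI component states.
; Sight tracks Human-tagged actors, dropping dead ones, while a looping timer is meant to retarget TargetActor to the closest.
; Lost targets linger until a memory timer expires them, falling back to TargetLocation as the last few are removed.
; Hearing sets TargetLocation only while nothing is in sight.
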(event OnTargetPerceptionUpdated(AIPerception)
  (params (Actor :type Actor%20Object%20Reference) (Stimulus :type AI%20Stimulus%20Structure))
  ;[0 0 0] Perception Update
  (CallFunction|Sight Actor Stimulus)
  (CallFunction|Hearing Actor Stimulus))

(event Custom|Actors%20in%20Sight%20-%20Distance%20Check
  ;[0 0 0] Actors in Sight - Distance Check
  (bind _returnvalue (Utilities|Time|SetTimerbyEvent (delegate Custom|CustomEvent_0) 3.0 true))
  (Variables|Don'tEdit|SetDistance%20Check%20-%20Timer _returnvalue))

(event Custom|CustomEvent_0
  ;[0 0 0] Actors in Sight - Distance Check
  (CallFunction|CheckActorsinSight))

(event Custom|Check%20Actors%20in%20Sight
  ;[0 0 0] Actors in Sight - Distance Check
  (if (not (Utilities|Map|IsEmpty (Variables|Don'tEdit|GetActors%20in%20Sight)))
    (bind _closest_actor (CallFunction|CheckDistance))
    (AI|Components|Blackboard|SetValueasObject (Variables|Default|GetBlackboard) (Utilities|Name|MakeLiteralName "TargetActor") _closest_actor)))

(event Custom|Check%20AI%20Memory
  ;[0 0 0] Memory
  (bind _returnvalue (Utilities|Time|SetTimerbyFunctionName 0 "Memory" 4.0 true))
  (Variables|Don'tEdit|SetMemory%20-%20Timer _returnvalue))

(event EventPossess
  (params (PossessedPawn :type Pawn%20Object%20Reference))
  (bind _returnvalue (Actor|GetComponentbyClass PossessedPawn "/Game/ZomTech/Blueprints/Components/BP_Zombie_AI_Component.BP_Zombie_AI_Component_C"))
  ;[0 0 0] Run Behavior Tree
  (Utilities|IsValid _returnvalue
    (:Is%20Valid
      (bind _output_get (Variables|Default|SetAI%20Component _returnvalue))
      (AI|RunBehaviorTree "/Game/ZomTech/Blueprints/AI/BT_Zombie_AI.BT_Zombie_AI")
      (Utilities|FlowControl|Delay 1.0)
      (Default|AICharacterPossessed _output_get))))

(fn ConstructionScript)

(fn Sight
  (params (Actor :type Actor%20Object%20Reference) (Stimulus :type AI%20Stimulus%20Structure))
  ;[0 0 0] Sight
  (LocalVariables|SetActor%20L Actor)
  (bind _output_get (LocalVariables|SetStimulus%20L Stimulus))
  (bind _returnvalue (Class|AIPerceptionSystem|GetSenseClassforStimulus _output_get))
  (if (== _returnvalue "/Script/AIModule.AISense_Sight")
    ;;[0 0 0] Is Human?
    (if (Actor|ActorHasTag (LocalVariables|GetActor%20L) "Human")
      (Utilities|IsValid (Actor|GetComponentbyClass (LocalVariables|GetActor%20L) "/Game/ZomTech/Blueprints/Components/BP_ZomTech_Character_Component.BP_ZomTech_Character_Component_C")
        (:Is%20Valid
          (if (Variables|/Game/ZomTech/Blueprints/Components/BP_ZomTech_Character_Component.BP_ZomTech_Character_Component_C|GetDead (Actor|GetComponentbyClass (LocalVariables|GetActor%20L) "/Game/ZomTech/Blueprints/Components/BP_ZomTech_Character_Component.BP_ZomTech_Character_Component_C"))
            (if (Utilities|Map|Contains (Variables|Don'tEdit|GetActors%20in%20Sight) (LocalVariables|GetActor%20L))
              (CallFunction|RemoveActorsinSight (Utilities|Array|MakeArray (LocalVariables|GetActor%20L)))
              (return)
              (else
                (return)))
            (else
              _)))
        (:Is%20Not%20Valid
          _))
      (if (Utilities|Struct|BreakAIStimulus _output_get)
        (if (Utilities|Map|IsEmpty (Variables|Don'tEdit|GetActors%20in%20Sight))
          (CallFunction|ActorsinSight-DistanceCheck)
          (Utilities|Map|Add (Variables|Don'tEdit|GetActors%20in%20Sight) (LocalVariables|GetActor%20L) (LocalVariables|GetStimulus%20L))
          (Utilities|Time|ClearandInvalidateTimerbyHandle (Variables|Don'tEdit|GetMemory%20-%20Timer))
          ;;[0 0 0] Set Target Actor
          (AI|Components|Blackboard|SetValueasObject (Variables|Default|GetBlackboard) (Utilities|Name|MakeLiteralName "TargetActor") (select (Utilities|Struct|BreakAIStimulus (LocalVariables|GetStimulus%20L)) (LocalVariables|GetActor%20L) 0))
          (if (Utilities|Struct|BreakAIStimulus (LocalVariables|GetStimulus%20L))
            (Default|SetCurrentAIState (Variables|Default|GetAI%20Component) "NewEnumerator1")
            (return)
            (else
              (AI|Components|Blackboard|SetValueasVector (Variables|Default|GetBlackboard) (Utilities|Name|MakeLiteralName "TargetLocation") (Utilities|Struct|BreakAIStimulus (LocalVariables|GetStimulus%20L)))
              (Default|SetCurrentAIState (Variables|Default|GetAI%20Component) "NewEnumerator3")
              (return)))
          (else
            (Utilities|Map|Remove (Variables|Don'tEdit|GetActors%20To%20Remove) (LocalVariables|GetActor%20L))
            (Utilities|Map|Add (Variables|Don'tEdit|GetActors%20in%20Sight) (LocalVariables|GetActor%20L) (LocalVariables|GetStimulus%20L))
            (Default|SetCurrentAIState (Variables|Default|GetAI%20Component) "NewEnumerator1")
            (return)))
        (else
          (Utilities|Map|Add (Variables|Don'tEdit|GetActors%20To%20Remove) (LocalVariables|GetActor%20L) (+ (Actor|GetGameTimeSinceCreation) (Variables|Settings|GetPlayer%20-%20MemoryTimeout)))
          (CallFunction|CheckAIMemory)
          (if (Utilities|Map|IsEmpty (Variables|Don'tEdit|GetActors%20in%20Sight))
            (Utilities|Time|ClearandInvalidateTimerbyHandle (Variables|Don'tEdit|GetDistance%20Check%20-%20Timer))
            (return)
            (else
              (CallFunction|CheckActorsinSight)
              (return)))))
      (else
        _)))
  (return))

(fn Hearing
  (params (Actor :type Actor%20Object%20Reference) (Stimulus :type AI%20Stimulus%20Structure))
  ;[0 0 0] Sight
  (LocalVariables|SetActor%20L Actor)
  (bind _output_get (LocalVariables|SetStimulus%20L Stimulus))
  (bind _returnvalue (Class|AIPerceptionSystem|GetSenseClassforStimulus _output_get))
  (if (== _returnvalue "/Script/AIModule.AISense_Hearing")
    (if (Utilities|Map|IsEmpty (Variables|Don'tEdit|GetActors%20in%20Sight))
      (AI|Components|Blackboard|SetValueasVector (Variables|Default|GetBlackboard) (Utilities|Name|MakeLiteralName "TargetLocation") (Utilities|Struct|BreakAIStimulus (LocalVariables|GetStimulus%20L)))
      (Default|SetCurrentAIState (Variables|Default|GetAI%20Component) "NewEnumerator5")
      (return)
      (else
        (return)))
    (else
      (return))))

(fn CheckDistance
  ;[0 0 0] Check Distance
  (bind _keys (Utilities|Map|Keys (Variables|Don'tEdit|GetActors%20in%20Sight)))
  (for _array_element _keys
    (Utilities|IsValid _array_element
      (:Is%20Valid
        (if (< (Transformation|GetDistanceTo _array_element (Pawn|GetControlledPawn)) (LocalVariables|GetDistance%20L))
          (LocalVariables|SetDistance%20L (Transformation|GetDistanceTo _array_element (Pawn|GetControlledPawn)))
          (LocalVariables|SetClosest%20Actor%20L _array_element)))))
  (return (LocalVariables|GetClosest%20Actor%20L)))

(fn Memory
  ;[0 0 0] Check Memory
  (bind _keys (Utilities|Map|Keys (Variables|Don'tEdit|GetActors%20To%20Remove)))
  (for _array_element _keys
    (Utilities|IsValid _array_element
      (:Is%20Valid
        (if (< (.Value (Utilities|Map|Find (Variables|Don'tEdit|GetActors%20To%20Remove) _array_element)) (Actor|GetGameTimeSinceCreation))
          (Utilities|Array|AddUnique (LocalVariables|GetActors%20to%20Remove%20L) _array_element)))))
  (CallFunction|RemoveActorsinSight (LocalVariables|GetActors%20to%20Remove%20L))
  (return))

(fn RemoveActorsinSight
  (params (Actors%20To%20Remove :type Array%20of%20Actor%20Object%20References))
  ;[0 0 0] Remove Actors in Sight
  (if (Utilities|Map|IsEmpty (Variables|Don'tEdit|GetActors%20in%20Sight))
    (Utilities|Time|ClearandInvalidateTimerbyHandle (Variables|Don'tEdit|GetMemory%20-%20Timer))
    (Utilities|Time|ClearandInvalidateTimerbyHandle (Variables|Don'tEdit|GetDistance%20Check%20-%20Timer))
    (return)
    (else
      (for _array_element Actors%20To%20Remove
        (if (> (Utilities|Map|Length (Variables|Don'tEdit|GetActors%20in%20Sight)) 2)
          (Utilities|Map|Remove (Variables|Don'tEdit|GetActors%20To%20Remove) _array_element)
          (Utilities|Map|Remove (Variables|Don'tEdit|GetActors%20in%20Sight) _array_element)
          (else
            (AI|Components|Blackboard|SetValueasVector (Variables|Default|GetBlackboard) (Utilities|Name|MakeLiteralName "TargetLocation") (Transformation|GetActorLocation _array_element))
            (Default|SetCurrentAIState (Variables|Default|GetAI%20Component) "NewEnumerator3")
            (Utilities|Map|Remove (Variables|Don'tEdit|GetActors%20To%20Remove) _array_element)
            (Utilities|Map|Remove (Variables|Don'tEdit|GetActors%20in%20Sight) _array_element))))
      (if (Utilities|Map|IsEmpty (Variables|Don'tEdit|GetActors%20in%20Sight))
        (AI|Components|Blackboard|SetValueasObject (Variables|Default|GetBlackboard) (Utilities|Name|MakeLiteralName "TargetActor") 0)
        (return)
        (else
          (return))))))