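; Player controller component that manages a ZomTech player's health, stamina, ammo and Left Shift sprinting.
; Sprint sets walk speed locally and on the server, where looping timers drain or regenerate stamina and exhaustion forces walking.
; RepNotify functions push stat changes to the local controller's HUD bars.
; Zero health flags the character component dead and restarts the level through player 0's BP_Human.
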(event Custom|Initialize
  (params (HUD :type WB%20HUD%20Object%20Reference))
  ;[0 0 0] Initialize
  (Variables|Default|SetHUD HUD)
  (CallFunction|SetStats-Server))

(event Custom|Set%20Stats%20-%20Server
  ;[0 0 0] Initialize
  (Variables|Attributes|SetCurrent%20Health (Variables|Attributes|GetMax%20Health))
  (Variables|Attributes|SetCurrent%20Stamina (Variables|Attributes|GetMax%20Stamina))
  (Variables|Gun|SetCurrentBullets 1))

(event Custom|AddBullets
  (params (DeltaBullets :type Integer))
  ;[1 1 1] Add Bullets Here
  (Variables|Gun|SetCurrentBullets (Math|Integer|Clamp(Integer) (+ DeltaBullets (Variables|Gun|GetCurrentBullets)) 0 (Variables|Gun|GetMaxBulletCapacity))))

(event Custom|Set%20Max%20Walk%20Speed%20-%20Server
  (params (Max%20Walk%20Speed :type Float%20%28single-precision%29) (Sprint :type Boolean))
  ;[0 0 0] Set Max Walk Speed - Server
  (if Sprint
    (CallFunction|SetMaxWalkSpeed Max%20Walk%20Speed)
    (Utilities|Time|ClearandInvalidateTimerbyHandle (Variables|Default|GetIncrease%20Stamina%20-%20Timer))
    (bind _returnvalue (Utilities|Time|SetTimerbyFunctionName 0 "Decrease Stamina" 0.1 true))
    (Variables|Default|SetDecrease%20Stamina%20-%20Timer _returnvalue)
    (else
      (CallFunction|SetMaxWalkSpeed Max%20Walk%20Speed)
      (Utilities|Time|ClearandInvalidateTimerbyHandle (Variables|Default|GetDecrease%20Stamina%20-%20Timer))
      (bind _returnvalue_2 (Utilities|Time|SetTimerbyFunctionName 0 "Increase Stamina" 0.1 true))
      (Variables|Default|SetIncrease%20Stamina%20-%20Timer _returnvalue_2))))

(event Custom|No%20Stamina
  ;[0 0 0] No Stamina
  (CallFunction|NoStamina-Client)
  (CallFunction|SetMaxWalkSpeed-Server (Variables|Attributes|GetWalk%20Speed) false))

(event Custom|No%20Stamina%20-Client
  ;[0 0 0] No Stamina
  (CallFunction|SetMaxWalkSpeed (Variables|Attributes|GetWalk%20Speed)))

(event Input|KeyboardEvents|LeftShift
  (params (Key :type Key%20Structure))
  (bind _sprint_speed (Variables|Attributes|GetSprint%20Speed))
  (bind _walk_speed (Variables|Attributes|GetWalk%20Speed))
  ;[0 0 0] Sprint
  (:Pressed
    (CallFunction|SetMaxWalkSpeed _sprint_speed)
    (CallFunction|SetMaxWalkSpeed-Server _sprint_speed true))
  (:Released
    (CallFunction|SetMaxWalkSpeed _walk_speed)
    (CallFunction|SetMaxWalkSpeed-Server _walk_speed false)))

(fn DecreaseHealth
  (params (Amount :type Float%20%28double-precision%29))
  ;[0 0 0] Decrease Health
  (Variables|/Game/ZomTech/Blueprints/Components/BP_ZomTech_Character_Component.BP_ZomTech_Character_Component_C|GetAs%20Character (Variables|Default|GetZomTech_Character_Component)
    (:then
      (if (> (Variables|Attributes|GetCurrent%20Health) 0.0)
        (if (<= (- (Variables|Attributes|GetCurrent%20Health) Amount) 0.0)
          (Variables|Attributes|SetCurrent%20Health 0.0)
          (Variables|/Game/ZomTech/Blueprints/Components/BP_ZomTech_Character_Component.BP_ZomTech_Character_Component_C|SetDead (Variables|Default|GetZomTech_Character_Component) true)
          (bind _asbp_human (Utilities|Casting|CastToBP_Human (Game|GetPlayerCharacter 0)))
          (Default|RestartLevel _asbp_human)
          (else
            (Variables|Attributes|SetCurrent%20Health (- (Variables|Attributes|GetCurrent%20Health) Amount))))))
    (:else)))

(fn OnRepCurrentHealth
  ;[0 0 0] On Rep Current Health
  (Utilities|IsLocalController
    (:true
      (bind _hud (Variables|Default|GetHUD)
        (:then
          (bind _wb_health (Variables|/Game/ZomTech/Blueprints/Widgets/WB_HUD.WB_HUD_C|GetWB_Health _hud)
            (:then
              (Default|UpdatePercent _wb_health (Variables|Attributes|GetCurrent%20Health) (Variables|Attributes|GetMax%20Health)))
            (:else)))
        (:else)))))

(fn OnRepCurrentStamina
  ;[0 0 0] On Rep Current Stamina
  (Utilities|IsLocalController
    (:true
      (bind _hud (Variables|Default|GetHUD)
        (:then
          (bind _wb_stamina (Variables|/Game/ZomTech/Blueprints/Widgets/WB_HUD.WB_HUD_C|GetWB_Stamina _hud)
            (:then
              (Default|UpdatePercent _wb_stamina (Variables|Attributes|GetCurrent%20Stamina) (Variables|Attributes|GetMax%20Stamina)))
            (:else)))
        (:else)))))

(fn SetMaxWalkSpeed
  (params (Max%20Walk%20Speed :type Float%20%28single-precision%29))
  ;[0 0 0] Set Max Walk Speed
  (bind _zomtech_character_component (Variables|Default|GetZomTech_Character_Component)
    (:then
      (Variables|/Script/Engine.CharacterMovementComponent|SetMaxWalkSpeed (Variables|/Game/ZomTech/Blueprints/Components/BP_ZomTech_Character_Component.BP_ZomTech_Character_Component_C|GetCharacter%20Movement _zomtech_character_component) Max%20Walk%20Speed))
    (:else)))

(fn DecreaseStamina
  ;[0 0 0] Decrease Stamina
  (if (>= (- (Variables|Attributes|GetCurrent%20Stamina) 2.0) 0.0)
    (Variables|Attributes|SetCurrent%20Stamina (- (Variables|Attributes|GetCurrent%20Stamina) 2.0))
    (else
      (Variables|Attributes|SetCurrent%20Stamina 0.0)
      (CallFunction|NoStamina))))

(fn IncreaseStamina
  ;[0 0 0] Increase Stamina
  (if (>= (+ (Variables|Attributes|GetCurrent%20Stamina) 3.0) 1e+02)
    (Variables|Attributes|SetCurrent%20Stamina 1e+02)
    (else
      (Variables|Attributes|SetCurrent%20Stamina (+ (Variables|Attributes|GetCurrent%20Stamina) 3.0)))))

(fn HasAmmo
  (return (or (> (Variables|Gun|GetCurrentBullets) 0.0) (Variables|Gun|GetbHasInfiniteAmmo))))

(fn OnRepCurrentBullets
  (Utilities|IsLocalController
    (:true
      (bind _hud (Variables|Default|GetHUD)
        (:then
          (bind _ammo (Variables|/Game/ZomTech/Blueprints/Widgets/WB_HUD.WB_HUD_C|GetAmmo _hud)
            (:then
              (Default|UpdatePercent _ammo (Math|Conversions|ToFloat(Integer) (Variables|Gun|GetCurrentBullets)) (Math|Conversions|ToFloat(Integer) (Variables|Gun|GetMaxBulletCapacity))))
            (:else)))
        (:else)))))

(fn IncreaseHealth
  (params (Amount :type Float%20%28double-precision%29))
  ;[0 0 0] Decrease Health
  (Variables|/Game/ZomTech/Blueprints/Components/BP_ZomTech_Character_Component.BP_ZomTech_Character_Component_C|GetAs%20Character (Variables|Default|GetZomTech_Character_Component)
    (:then
      (Variables|Attributes|SetCurrent%20Health (Math|Float|Clamp(Float) (+ Amount (Variables|Attributes|GetCurrent%20Health)) 0.0 (Variables|Attributes|GetMax%20Health))))
    (:else)))

(fn IsatMaxAmmo
  (return (== (Variables|Gun|GetCurrentBullets) (Variables|Gun|GetMaxBulletCapacity))))

(fn IsatMaxHealth
  (return (== (Variables|Attributes|GetCurrent%20Health) (Variables|Attributes|GetMax%20Health))))