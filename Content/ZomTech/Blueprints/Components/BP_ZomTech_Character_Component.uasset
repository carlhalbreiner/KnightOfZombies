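; ZomTech character component that handles aiming and death for its owning Character, caching the character and its movement component on BeginPlay.
; Right mouse toggles aiming locally and via a server event, messages the owner to update field of view, and switches between movement-facing and slower controller-facing rotation.
; The Dead RepNotify triggers death, which ragdolls the mesh, relaxes capsule and camera collision, stops movement and disables input.
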(event Custom|Character%20Dead
  (bind _as_character (Variables|Default|GetAs%20Character))
  (bind _capsulecomponent (Variables|/Script/Engine.Character|GetCapsuleComponent _as_character))
  ;[0 0 0] Dead
  (bind _as_character_2 (Variables|Default|GetAs%20Character)
    (:then
      (Physics|SetSimulatePhysics (Variables|/Script/Engine.Character|GetMesh _as_character_2) true)
      (Collision|SetCollisionProfileName (Variables|/Script/Engine.Character|GetMesh _as_character_2) "Ragdoll" true :!class /Script/Engine.PrimitiveComponent)
      (Collision|SetCollisionResponsetoChannel _capsulecomponent "ECC_Pawn" "ECR_Ignore")
      (Collision|SetCollisionResponsetoChannel _capsulecomponent "ECC_Camera" "ECR_Ignore")
      (Collision|SetCollisionResponsetoChannel _capsulecomponent "ECC_PhysicsBody" "ECR_Ignore")
      (Collision|SetCollisionResponsetoChannel _capsulecomponent "ECC_Visibility" "ECR_Ignore")
      (Components|Movement|StopMovementImmediately (Variables|/Script/Engine.Character|GetCharacterMovement _as_character))
      (Input|DisableInput _as_character (.AsPlayer%20Controller (Utilities|Casting|CastToPlayerController (Pawn|GetController (.AsPawn (Utilities|Casting|CastToPawn (Components|GetOwner))))))))
    (:else)))

(event Custom|Set%20Aiming%20-%20Server
  (params (Aiming :type Boolean))
  ;[0 0 0] Set Aiming - Server
  (bind _output_get (Variables|Default|SetAiming Aiming))
  (CallFunction|SetAiming _output_get))

(event EventBeginPlay
  ;[0 0 0] Begin Play
  (bind _ascharacter (Utilities|Casting|CastToCharacter (Components|GetOwner)))
  (Variables|Default|SetAs%20Character _ascharacter)
  (Variables|Default|SetCharacter%20Movement (Variables|/Script/Engine.Character|GetCharacterMovement (Variables|Default|GetAs%20Character))))

(event Input|MouseEvents|RightMouseButton
  (params (Key :type Key%20Structure))
  (bind _returnvalue (Components|GetOwner))
  ;[0 0 0] Aiming
  (:Pressed
    (CallFunction|SetAiming-Server true)
    (Class|BPHumanInterface|UpdateFieldOfView(Message) _returnvalue true)
    (CallFunction|SetAiming true))
  (:Released
    (CallFunction|SetAiming-Server false)
    (Class|BPHumanInterface|UpdateFieldOfView(Message) _returnvalue false)
    (CallFunction|SetAiming false)))

(fn SetAiming
  (params (Aiming :type Boolean))
  (bind _character_movement (Variables|Default|GetCharacter%20Movement))
  ;[0 0 0] Set Aiming
  (if Aiming
    (Variables|/Script/Engine.CharacterMovementComponent|SetbOrientRotationToMovement (Variables|Default|GetCharacter%20Movement) false)
    (Variables|/Script/Engine.CharacterMovementComponent|SetbUseControllerDesiredRotation (Variables|Default|GetCharacter%20Movement) true)
    (Variables|/Script/Engine.CharacterMovementComponent|SetRotationRate _character_movement "0,120.000000, 0")
    (else
      (Variables|/Script/Engine.CharacterMovementComponent|SetbOrientRotationToMovement (Variables|Default|GetCharacter%20Movement) true)
      (Variables|/Script/Engine.CharacterMovementComponent|SetbUseControllerDesiredRotation (Variables|Default|GetCharacter%20Movement) false)
      (Variables|/Script/Engine.CharacterMovementComponent|SetRotationRate _character_movement "0,360.000000, 0"))))

(fn OnRepDead
  ;[0 0 0] Dead
  (CallFunction|CharacterDead))