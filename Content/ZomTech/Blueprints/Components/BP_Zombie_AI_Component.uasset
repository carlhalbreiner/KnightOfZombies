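; Zombie AI component that manages a Character's state, montages, melee attacks, health and death in multiplayer.
; State changes update the AI_State blackboard key, and multicast montages are picked from the current state.
; Attacks run a looping timer of sphere traces at head or hand sockets until a hit, applying damage only on the server.
; Zero health stops the brain logic, while RepNotifies trigger ragdoll and sync the random blendspace variant.
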(event Custom|AI%20Character%20Possessed
  ;[0 0 0] AI Character Possessed
  (bind _ascharacter (Utilities|Casting|CastToCharacter (Components|GetOwner)))
  (Variables|Don'tEdit|SetAs%20Character _ascharacter)
  (CallFunction|SetCurrentAIState (Variables|State|GetStart%20State))
  (CallFunction|SetRandomBlendspace))

(event Custom|Play%20Montage%20-%20Multicast
  ;[0 0 0] Play Montage - Multicast
  (bind _output_get (Variables|Don'tEdit|SetCurrent%20Montage (Utilities|Select :Index (Variables|State|GetCurrent%20State) :NewEnumerator4 0 :NewEnumerator0 0 :NewEnumerator1 (.OutItem (Utilities|Array|Random (Variables|Settings|Montage|GetAttack%20Montages))) :NewEnumerator2 0 :NewEnumerator3 (.OutItem (Utilities|Array|Random (Variables|Settings|Montage|GetSearch%20Montages))) :NewEnumerator5 "/Game/ZomTech/Animations/AM_Search.AM_Search" :NewEnumerator7 0)))
  (Utilities|IsValid _output_get
    (:Is%20Valid
      (Animation|Montage|PlayMontage (Variables|/Script/Engine.Character|GetMesh (Variables|Don'tEdit|GetAs%20Character)) _output_get
        (:OnCompleted
          (Default|CallOnComplete(Montage))
          (Variables|Don'tEdit|SetCurrent%20Montage 0))))
    (:Is%20Not%20Valid
      (Default|CallOnComplete(Montage)))))

(event Custom|Stop%20Montage%20-%20Multicast
  ;[0 0 0] Stop Montage - Multicast
  (Animation|StopAnimMontage (Variables|Don'tEdit|GetAs%20Character) (Variables|Don'tEdit|GetCurrent%20Montage))
  (Variables|Don'tEdit|SetCurrent%20Montage 0))

(event Custom|Attacking%20-%20Multicast
  (params (Attack%20Type :type E_AI_Attack%20Enum :default "NewEnumerator0") (Active :type Boolean))
  ;[0 0 0] Attacking
  (Variables|Don'tEdit|SetCurrent%20Attack%20Type Attack%20Type)
  (if Active
    (bind _returnvalue (Utilities|Time|SetTimerbyEvent (delegate Custom|CustomEvent_0) 0.06 true))
    (Variables|Don'tEdit|SetAttack%20-%20Timer _returnvalue)
    (else
      (Utilities|Time|ClearandInvalidateTimerbyHandle (Variables|Don'tEdit|GetAttack%20-%20Timer)))))

(event Custom|CustomEvent_0
  (bind _attack_sounds (Variables|Settings|GetAttack%20Sounds))
  ;[0 0 0] Attacking
  (bind (_outhit _hit) (CallFunction|SphereTrace (Variables|Don'tEdit|GetCurrent%20Attack%20Type)))
  (if _hit
    (bind _hit_effect (Variables|Settings|GetHit%20Effect)
      (:then
        ;;[0 0 0] Spawn Hit Effect
        (Niagara|SpawnSystematLocation _hit_effect (.ImpactPoint (Collision|BreakHitResult _outhit))))
      (:else
        _))
    (Utilities|Time|ClearandInvalidateTimerbyHandle (Variables|Don'tEdit|GetAttack%20-%20Timer))
    (if (Utilities|Array|IsEmpty _attack_sounds)
      _
      (else
        (Audio|PlaySoundatLocation (.OutItem (Utilities|Array|Random _attack_sounds)) (Transformation|GetActorLocation (Variables|Don'tEdit|GetAs%20Character)) "0, 0, 0" 1.0 1.0 0.0 0 0 0 0)))
    ;;[0 0 0] Apply Damage - If Server
    (Utilities|IsServer
      (:true
        (Game|Damage|ApplyDamage (.HitActor (Collision|BreakHitResult _outhit)) 15.0 0 (Variables|Don'tEdit|GetAs%20Character))))))

(event Custom|AI%20Dead
  (bind _as_character (Variables|Don'tEdit|GetAs%20Character))
  (bind _as_character_2 (Variables|Don'tEdit|GetAs%20Character))
  (bind _mesh (Variables|/Script/Engine.Character|GetMesh _as_character_2))
  (bind _capsulecomponent (Variables|/Script/Engine.Character|GetCapsuleComponent _as_character))
  ;[0 0 0] Dead
  (Physics|SetSimulatePhysics _mesh true)
  (Collision|SetCollisionProfileName _mesh "Ragdoll" true :!class /Script/Engine.PrimitiveComponent)
  (Collision|SetCollisionResponsetoChannel _capsulecomponent "ECC_Pawn" "ECR_Ignore")
  (Collision|SetCollisionResponsetoChannel _capsulecomponent "ECC_Camera" "ECR_Ignore")
  (Collision|SetCollisionResponsetoChannel _capsulecomponent "ECC_PhysicsBody" "ECR_Ignore")
  (Components|Movement|StopMovementImmediately (Variables|/Script/Engine.Character|GetCharacterMovement (Variables|Don'tEdit|GetAs%20Character)))
  (Input|DisableInput (Variables|Don'tEdit|GetAs%20Character) (.AsPlayer%20Controller (Utilities|Casting|CastToPlayerController (Pawn|GetController (.AsPawn (Utilities|Casting|CastToPawn (Components|GetOwner))))))))

(event Custom|AI%20Dead%20-%20Server
  ;[0 0 0] Dead
  (Variables|Don'tEdit|SetDead true)
  (AI|Logic|StopLogic (Variables|/Script/AIModule.AIController|GetBrainComponent (AI|GetAIController (Variables|Don'tEdit|GetAs%20Character))) "Dead"))

(fn SetCurrentAIState
  (params (AI%20State :type E_AI_State%20Enum :default "NewEnumerator4"))
  ;[0 0 0] Set Current AIState
  (LocalVariables|SetAI%20State%20L AI%20State)
  (if (not (Utilities|Enum|Equal(Enum) (LocalVariables|GetAI%20State%20L) (Variables|State|GetCurrent%20State)))
    (bind _as_character (Variables|Don'tEdit|GetAs%20Character)
      (:then
        (Utilities|IsValid (AI|GetBlackboard (Pawn|GetController _as_character))
          (:Is%20Valid
            (bind _output_get (Variables|State|SetCurrent%20State (LocalVariables|GetAI%20State%20L)))
            (AI|Components|Blackboard|SetValueasEnum (AI|GetBlackboard (Pawn|GetController _as_character)) (Utilities|Name|MakeLiteralName "AI_State") _output_get))))
      (:else))))

(fn SphereTrace
  (params (Attack%20Type :type E_AI_Attack%20Enum :default "NewEnumerator0"))
  (bind _head (Variables|Sockets|GetHead))
  (bind _left_hand (Variables|Sockets|GetLeft%20Hand))
  (bind _right_hand (Variables|Sockets|GetRight%20Hand))
  (bind _as_character (Variables|Don'tEdit|GetAs%20Character))
  (bind _returnvalue (Utilities|Select :Index Attack%20Type :NewEnumerator0 _head :NewEnumerator1 _left_hand :NewEnumerator2 _right_hand))
  (bind _mesh (Variables|/Script/Engine.Character|GetMesh _as_character))
  (bind _returnvalue_2 (Transformation|GetSocketLocation _mesh _returnvalue))
  ;[0 0 0] Sphere Trace
  (bind (_outhit _returnvalue_3) (Collision|SphereTraceByChannel _returnvalue_2 (+ _returnvalue_2 (* (Transformation|GetActorForwardVector (Variables|Don'tEdit|GetAs%20Character)) 7.0)) 25.0 "TraceTypeQuery3" false (Utilities|Array|MakeArray (Components|GetOwner)) "None"))
  (return _outhit _returnvalue_3))

(fn OnRepBlendspaceIndex
  ;[0 0 0] Set Blendspace
  (Class|BPZombieInterface|SetBlendspace(Message) (Components|SkeletalMesh|GetAnimInstance (Variables|/Script/Engine.Character|GetMesh (Variables|Don'tEdit|GetAs%20Character))) (Variables|Don'tEdit|GetBlendspace%20Index)))

(fn SetRandomBlendspace
  ;[0 0 0] Set Random Blendspace
  (bind _output_get (Variables|Don'tEdit|SetBlendspace%20Index (Math|Random|RandomIntegerinRange 0 (Variables|Settings|GetMax%20Blendspaces))))
  (Class|BPZombieInterface|SetBlendspace(Message) (Components|SkeletalMesh|GetAnimInstance (Variables|/Script/Engine.Character|GetMesh (Variables|Don'tEdit|GetAs%20Character))) _output_get))

(fn DecreaseHealth
  (params (Amount :type Float%20%28double-precision%29))
  ;[0 0 0] Decrease Health
  (if (Variables|Don'tEdit|GetDead)
    (return true)
    (elif (<= (- (Variables|Settings|GetCurrent%20Health) Amount) 0.0)
      (Variables|Settings|SetCurrent%20Health 0.0)
      (CallFunction|AIDead-Server)
      (return true)
      (else
        (Variables|Settings|SetCurrent%20Health (- (Variables|Settings|GetCurrent%20Health) Amount))
        (return false)))))

(fn OnRepCurrentHealth
  ;[0 0 0] AI Dead
  (if (<= (Variables|Settings|GetCurrent%20Health) 0.0)
    (CallFunction|AIDead)))